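; Knockable component that lets its owning Character be knocked back, softened by a resistance value.
; Knockback scales the given strength by one minus the clamped KnockbackResist, stops the character's movement immediately, then calls LaunchCharacter with XY override.
; Only the X and Z components of the strength feed the launch; Y is left unset.
; Owners that are not Characters are ignored, and the event graph is unused.
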(event EventBeginPlay)

(event EventTick
  (params (DeltaSeconds :type Float%20%28single-precision%29)))

(fn Knockback
  (params (Strength :type Vector))
  (bind (_x _y _z) (Math|Vector|BreakVector Strength))
  (LocalVariables|SetMultiplier (- 1.0 (Math|Float|Clamp(Float) (Variables|Default|GetKnockbackResist))))
  (bind _ascharacter (Utilities|Casting|CastToCharacter (Components|GetOwner)))
  (Components|Movement|StopMovementImmediately (Variables|/Script/Engine.Character|GetCharacterMovement _ascharacter))
  (Character|LaunchCharacter _ascharacter (Math|Vector|MakeVector (* _x (LocalVariables|GetMultiplier)) 0.0 (* _z (LocalVariables|GetMultiplier))) true false))