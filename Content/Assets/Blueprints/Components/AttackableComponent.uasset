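; AttackableComponent is an actor component that gives its owner a light attack through the Gameplay Ability System.
; On BeginPlay it grants the attack ability class to the owner's Ability System Component and stores the spec handle.
; When the light attack input starts, it tries to activate that ability, then sends the owner a tagged gameplay event naming the owner as instigator.
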(event Input|EnhancedActionEvents|EnhancedInputActionLightAttachAction
  (params (ActionValue :type Boolean) (ElapsedSeconds :type Float%20%28double-precision%29) (TriggeredSeconds :type Float%20%28double-precision%29) (InputAction :type Input%20Action%20Object%20Reference :default "/Game/Assets/Input/LightAttachAction.LightAttachAction"))
  (bind _returnvalue (Components|GetOwner))
  (bind _event_tag (Variables|Default|GetEvent%20Tag))
  ;[0.15 0.15 0.15 0.5] Attack (GAS)
  (:Started
    (Class|AbilitySystemComponent|TryActivateAbility (Ability|GetAbilitySystemComponent _returnvalue) (Variables|Default|GetAttackAbility) true)
    (Ability|SendGameplayEventtoActor _returnvalue _event_tag (Utilities|Struct|MakeGameplayEventData _event_tag _returnvalue))))

(event EventBeginPlay
  (bind _returnvalue (GameplayAbilities|GiveAbility (Actor|GetComponentbyClass (Components|GetOwner) "/Script/GameplayAbilities.AbilitySystemComponent") (Variables|Default|GetAttackAbilityClass) 0 -1))
  (Variables|Default|SetAttackAbility _returnvalue))