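; Actor component that adds a charge-and-release ranged attack through the Gameplay Ability System.
; On BeginPlay it gets the owner's Ability System Component, grants the charging and shoot abilities, and stores their handles.
; Pressing the Heavy Attack input activates abilities by the charging tag, and completing it activates abilities by the shoot tag.
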(event Input|EnhancedActionEvents|EnhancedInputActionHeavyAttackAction
  (params (ActionValue :type Boolean) (ElapsedSeconds :type Float%20%28double-precision%29) (TriggeredSeconds :type Float%20%28double-precision%29) (InputAction :type Input%20Action%20Object%20Reference :default "/Game/Assets/Input/Actions/HeavyAttackAction.HeavyAttackAction"))
  ;[0.15 0.15 0.15 0.5] Use Ranged Weapon (GAS)
  (:Started
    (Abilities|TryActivateAbilitiesbyTag (Variables|Default|GetAbilityComponent) (Variables|Default|GetChargingTag) true))
  (:Completed
    (Abilities|TryActivateAbilitiesbyTag (Variables|Default|GetAbilityComponent) (Variables|Default|GetShootTag) true)))

(event EventBeginPlay
  (bind _output_get (Variables|Default|SetAbilityComponent (Ability|GetAbilitySystemComponent (Components|GetOwner))))
  (bind _returnvalue (GameplayAbilities|GiveAbility _output_get "/Game/Assets/Abilities/Redhat/ChargingAbility.ChargingAbility_C" 0 -1))
  (Variables|Default|SetchargeAbility _returnvalue)
  (bind _returnvalue_2 (GameplayAbilities|GiveAbility (Variables|Default|GetAbilityComponent) "/Game/Assets/Abilities/Redhat/ShootAbility.ShootAbility_C" 0 -1))
  (Variables|Default|SetshootAbility _returnvalue_2))