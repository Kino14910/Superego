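; Actor component that keeps the owner's camera at a height offset from the owner and makes meshes between them see-through.
; Each tick it sets only the camera's Z, then runs a visibility multi-trace from camera to owner.
; Newly hit meshes store slot 0's base material and get a dynamic instance of a transparent material.
; A set difference against the previous tick's hits finds uncovered meshes and restores their stored material.
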(event EventBeginPlay
  (Variables|Default|SetCamera (Actor|GetComponentbyClass (Components|GetOwner) "/Script/Engine.CameraComponent")))

(event EventTick
  (params (DeltaSeconds :type Float%20%28single-precision%29))
  (bind _returnvalue (Components|GetOwner))
  (bind _returnvalue_2 (Actor|GetComponentbyClass _returnvalue "/Script/Engine.CameraComponent"))
  (bind _returnvalue_3 (Transformation|GetWorldLocation _returnvalue_2))
  (Transformation|SetWorldLocation _returnvalue_2 (Math|Vector|MakeVector (.x _returnvalue_3) (.y _returnvalue_3) (+ (.z (Transformation|GetActorLocation _returnvalue)) (Variables|Default|GetoffsetZ))) false false)
  (CallFunction|Test))

(fn OnCovered
  (params (Dist :type Float%20%28double-precision%29) (Target :type Mesh%20Component%20Object%20Reference))
  (bind _returnvalue (Rendering|Material|GetBaseMaterial (Rendering|Material|GetMaterial Target 0)))
  (Utilities|Map|Add (Variables|Default|GetMaterials) Target _returnvalue)
  (bind _returnvalue_2 (Rendering|Material|CreateDynamicMaterialInstance "/Game/Assets/Materials/TransparentInst.TransparentInst" "None" "None" :!class /Script/Engine.KismetMaterialLibrary))
  (Rendering|Material|SetScalarParameterValue _returnvalue_2 "None" (/ Dist 1e+03) :!class /Script/Engine.MaterialInstanceDynamic)
  (Rendering|Material|SetMaterial Target 0 _returnvalue_2))

(fn OnVisible
  (params (Target :type Mesh%20Component%20Object%20Reference))
  (bind _materials (Variables|Default|GetMaterials))
  (Rendering|Material|SetMaterial Target 0 (.Value (Utilities|Map|Find _materials Target)))
  (Utilities|Map|Remove _materials Target))

(fn Test
  (bind _outhits (Collision|MultiLineTraceByChannel (Transformation|GetWorldLocation (Variables|Default|GetCamera)) (Transformation|GetActorLocation (Components|GetOwner)) "TraceTypeQuery1" false 0 "None"))
  (for _array_element _outhits
    (bind _asmesh_component (Utilities|Casting|CastToMeshComponent (.HitComponent (Collision|BreakHitResult _array_element))))
    (Utilities|Set|Add (Variables|Default|GetCoverd) _asmesh_component)
    (if (not (Utilities|Set|Contains (Variables|Default|GetCoverdOld) _asmesh_component))
      (CallFunction|OnCovered (.Distance (Collision|BreakHitResult _array_element)) _asmesh_component)))
  (bind _result (Utilities|Set|Difference (Variables|Default|GetCoverdOld) (Variables|Default|GetCoverd)))
  (bind _result_2 (Utilities|Set|ToArray _result))
  (for _array_element_2 _result_2
    (CallFunction|OnVisible _array_element_2))
  (Utilities|Set|Clear (Variables|Default|GetCoverdOld))
  (bind _result_3 (Utilities|Set|ToArray (Variables|Default|GetCoverd)))
  (for _array_element_3 _result_3
    (Utilities|Set|Add (Variables|Default|GetCoverdOld) _array_element_3))
  (Utilities|Set|Clear (Variables|Default|GetCoverd)))