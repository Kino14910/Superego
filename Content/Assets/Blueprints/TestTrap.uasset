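; TestTrap is a test trap actor that applies a gameplay effect to actors entering its box.
; On box overlap, it gets the other actor's Ability System Component, applies AttackEffect to it at a negative level and prints the overlapping component's name.
; Separately, overlapping the static mesh prints a debug message and sets a transparent stroke overlay material, which is cleared when the overlap ends.
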(event OnComponentBeginOverlap(Box)
  (params (OverlappedComponent :type Primitive%20Component%20Object%20Reference) (OtherActor :type Actor%20Object%20Reference) (OtherComp :type Primitive%20Component%20Object%20Reference) (OtherBodyIndex :type Integer) (bFromSweep :type Boolean) (SweepResult :type Hit%20Result%20Structure%20%28by%20ref%29))
  (GameplayEffects|ApplyGameplayEffectToSelf :self (Actor|GetComponentbyClass OtherActor "/Script/GameplayAbilities.AbilitySystemComponent") :GameplayEffectClass "/Game/Assets/PlayEffects/Redhood/AttackEffect.AttackEffect_C" :Level -2e+01)
  (Development|PrintString (Utilities|GetDisplayName OtherComp)))

(event OnComponentBeginOverlap(StaticMesh)
  (params (OverlappedComponent :type Primitive%20Component%20Object%20Reference) (OtherActor :type Actor%20Object%20Reference) (OtherComp :type Primitive%20Component%20Object%20Reference) (OtherBodyIndex :type Integer) (bFromSweep :type Boolean) (SweepResult :type Hit%20Result%20Structure%20%28by%20ref%29))
  (Development|PrintString "Hello")
  (Rendering|Material|SetOverlayMaterial (Variables|Default|GetStaticMesh) "/Game/Assets/Materials/TransparentStroke_Inst.TransparentStroke_Inst" :!class /Script/Engine.MeshComponent))

(event OnComponentEndOverlap(StaticMesh)
  (params (OverlappedComponent :type Primitive%20Component%20Object%20Reference) (OtherActor :type Actor%20Object%20Reference) (OtherComp :type Primitive%20Component%20Object%20Reference) (OtherBodyIndex :type Integer))
  (Rendering|Material|SetOverlayMaterial (Variables|Default|GetStaticMesh) 0 :!class /Script/Engine.MeshComponent))

(event EventBeginPlay)

(event Collision|EventActorBeginOverlap
  (params (OtherActor :type Actor%20Object%20Reference)))

(event EventTick
  (params (DeltaSeconds :type Float%20%28single-precision%29)))

(fn ConstructionScript)